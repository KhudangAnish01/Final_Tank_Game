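; Enemy tank Blueprint (NE2) that wires up its aiming, movement and health bar components on spawn.
; BeginPlay passes the barrel and turret to TankAiming and both tracks to TankMovement, then links the health bar widget back to this tank.
; Move Forward and Turn Right input axes are also bound, forwarding their values to the movement component's intend-move functions.
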(event EventBeginPlay
  (Class|TankAimingComponent|Initialse (Variables|Default|GetTankAiming) (Variables|Default|GetTankBarrel) (Variables|Default|GetTankTurret))
  (Class|TankMovementComponent|Inialise (Variables|Default|GetTankMovement) (Variables|Default|GetLeftTracK) (Variables|Default|GetRightTrack))
  (bind _ashealth_bar (Utilities|Casting|CastToHealthBar (UserInterface|GetUserWidgetObject (Variables|Default|GetHealtWidget))))
  (Variables|/Game/UI/HealthBar.HealthBar_C|SetMyTank _ashealth_bar self))

(event Input|AxisEvents|InputAxisMoveForward
  (params (AxisValue :type Float%20%28single-precision%29))
  ;[1 1 1] Movement Input Binding
  (Class|TankMovementComponent|IntendMoveForward (Variables|Default|GetTankMovement) AxisValue))

(event Input|AxisEvents|InputAxisTurnRight
  (params (AxisValue :type Float%20%28single-precision%29))
  ;[1 1 1] Movement Input Binding
  (Class|TankMovementComponent|IntendTurnRight (Variables|Default|GetTankMovement) AxisValue))

(fn ConstructionScript)